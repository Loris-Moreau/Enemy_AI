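; Patrol route actor for enemy behaviour that exposes waypoints along the PatrolRoute spline.
; IncrementPatrolRoute steps PatrolIndex by Direction, wrapping at the ends of closed loops and reversing direction at the ends of open splines to ping-pong.
; GetSplineWorldLocation returns the world position of the spline point at the current index.
; The index and direction are stored on the route itself.
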(event Custom|Increment%20Patrol%20Route
  (bind _patrol_route (Variables|Default|GetPatrol%20Route))
  (bind _returnvalue (Spline|GetNumberOfSplinePoints _patrol_route))
  (bind _output_get (Variables|Default|SetPatrol%20Index (+ (Variables|Default|GetPatrol%20Index) (Variables|Default|GetDirection))))
  (if (== _output_get (select (Class|SplineComponent|IsClosedLoop _patrol_route) _returnvalue (- _returnvalue 1)))
    (if (Class|SplineComponent|IsClosedLoop (Variables|Default|GetPatrol%20Route))
      (Variables|Default|SetPatrol%20Index 0)
      (else
        (Variables|Default|SetDirection -1)))
    (elif (== (Variables|Default|GetPatrol%20Index) 0)
      (if (Class|SplineComponent|IsClosedLoop (Variables|Default|GetPatrol%20Route))
        (Variables|Default|SetPatrol%20Index (Spline|GetNumberOfSplinePoints (Variables|Default|GetPatrol%20Route)))
        (else
          (Variables|Default|SetDirection 1))))))

(fn ConstructionScript)

(fn GetSplineWorldLocation
  (return (Spline|GetLocationatSplinePoint (Variables|Default|GetPatrol%20Route) (Variables|Default|GetPatrol%20Index) "World")))