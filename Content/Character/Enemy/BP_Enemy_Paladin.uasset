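; BP_Enemy_Paladin is an enemy character that punches the player and supplies movement and range data, likely for AI logic.
; Attack plays a punch montage, then deals small random whole-number damage to player 0 on completion, with no hit or range check.
; CallOnAttackEnd fires whether the montage completes or is interrupted.
; Helper functions return attack and strafe radii and the patrol path, and map a speed state to MaxWalkSpeed.
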(event Custom|Attack
  (Animation|Montage|PlayMontage (Variables|Character|GetMesh) "/Game/Characters/Mannequins/Animations/Montage_Punching.Montage_Punching"
    (:OnCompleted
      (bind _returnvalue (Game|Damage|ApplyDamage (Game|GetPlayerCharacter 0) (Math|Conversions|ToFloat(Integer) (Math|Float|Truncate (Math|Random|RandomFloatinRange 1.0 5.0))) 0 self "/Script/Engine.DamageType"))
      (Development|PrintString (Utilities|String|ToString(Float) _returnvalue) true false "(R=1.000000,G=0.000000,B=0.075629,A=1.000000)"))
    (:OnInterrupted
      (Development|PrintString "Montage Interupted" true true "(R=0.000000,G=0.650000,B=1.000000,A=1.000000)")))
  (Default|CallOnAttackEnd))

(event EventBeginPlay)

(fn ConstructionScript)

(fn GetIdealRange
  (return 2e+01 3.5e+02))

(fn GetPatrolPath
  (return (Variables|Default|GetPatrol%20Path)))

(fn SetMovementSpeed
  (params (Speeds :type E_Speeds%20Enum :default "NewEnumerator0"))
  (bind _output_get (Variables|/Script/Engine.CharacterMovementComponent|SetMaxWalkSpeed (Variables|Character|GetCharacterMovement) (Utilities|Select :Index Speeds :NewEnumerator0 0.0 :NewEnumerator1 2.2e+02 :NewEnumerator2 2.7e+02 :NewEnumerator3 3.5e+02)))
  (return _output_get))