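; Base enemy character that provides a melee punch attack, along with combat ranges, a patrol route and movement speed control.
; Attack plays a punch montage and, on completion, damages player 0 with no hit or range check and prints the result.
; Completed and interrupted montages both call OnAttackEnd.
; Getters expose attack and strafe radii and the patrol route, while SetMovementSpeed maps a speed enum to max walk speed.
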(event Custom|Attack
  (Animation|Montage|PlayMontage (Variables|Character|GetMesh) "/Game/Characters/Mannequins/Animations/Montage_Punching.Montage_Punching"
    (:OnCompleted
      (bind _returnvalue (Game|Damage|ApplyDamage (Game|GetPlayerCharacter 0) 1e+01 0 0 "/Script/Engine.DamageType"))
      (Development|PrintString (Utilities|String|ToString(Float) _returnvalue)))
    (:OnInterrupted
      _))
  (Default|CallOnAttackEnd))

(event EventBeginPlay)

(fn ConstructionScript)

(fn GetIdealRange
  (return 2e+01 3.5e+02))

(fn GetPatrolRoute
  (return (Variables|AI|GetPatrolRoute)))

(fn SetMovementSpeed
  (params (Speeds :type E_Speeds%20Enum :default "NewEnumerator0"))
  (bind _output_get (Variables|/Script/Engine.CharacterMovementComponent|SetMaxWalkSpeed (Variables|Character|GetCharacterMovement) (Utilities|Select :Index Speeds :NewEnumerator0 0.0 :NewEnumerator1 2.2e+02 :NewEnumerator2 2.7e+02 :NewEnumerator3 3.5e+02)))
  (return _output_get))