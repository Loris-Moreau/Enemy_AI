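; BP_PatrolRoute is an enemy patrol route that exposes the points of a spline as successive world-space destinations.
; IncrementPatrolRoute advances PatrolIndex by Direction, wrapping on closed-loop splines and reversing at either end of open ones for ping-pong movement.
; GetSplinePointAsWorldPosition returns the world location of the spline point at the current index.
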(event Custom|Increment%20Patrol%20Route
  (bind _spline (Variables|Default|GetSpline))
  (bind _returnvalue (Spline|GetNumberOfSplinePoints _spline))
  (bind _output_get (Variables|Default|SetPatrolIndex (+ (Variables|Default|GetPatrolIndex) (Variables|Default|GetDirection))))
  (if (== _output_get (select (Class|SplineComponent|IsClosedLoop (Variables|Default|GetSpline)) _returnvalue (- _returnvalue 1)))
    (if (Class|SplineComponent|IsClosedLoop (Variables|Default|GetSpline))
      (Variables|Default|SetPatrolIndex 0)
      (else
        (Variables|Default|SetDirection -1)))
    (elif (== (Variables|Default|GetPatrolIndex) 0)
      (if (Class|SplineComponent|IsClosedLoop (Variables|Default|GetSpline))
        (Variables|Default|SetPatrolIndex (Spline|GetNumberOfSplinePoints (Variables|Default|GetSpline)))
        (else
          (Variables|Default|SetDirection 1))))))

(fn ConstructionScript)

(fn GetSplinePointasWorldPosition
  (return (Spline|GetLocationatSplinePoint (Variables|Default|GetSpline) (Variables|Default|GetPatrolIndex) "World")))